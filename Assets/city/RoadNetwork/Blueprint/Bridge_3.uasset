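; Spline-driven bridge road builder that generates its meshes in the construction script.
; It resizes a per-point data array to match the spline, then lays one spline mesh per segment with that point's bank, width and thickness, optionally closing the loop.
; A final per-point pass optionally adds index text labels and offset, rotated support meshes.
; Guardrail flags are read but no guardrails are built.
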(event EventBeginPlay)

(event Collision|EventActorBeginOverlap
  (params (OtherActor :type Actor%20Object%20Reference)))

(fn ConstructionScript
  (bind _bridge_support_global_location_offset (Variables|Variables|GetBridge_Support_Global_Location_Offset))
  (bind (_x _y _z) (Math|Vector|BreakVector _bridge_support_global_location_offset))
  (Utilities|FlowControl|Sequence
    (:then_0
      ;[1 1 1] Store Number Of Splines Point
      (bind _output_get (Variables|Variables|SetNumberOfSplinePoints (Spline|GetNumberOfSplinePoints (Variables|Default|GetSpline)))))
    (:then_1
      (|BuildRoadArray _output_get))
    (:then_2
      (for _index (range 0 (select (Variables|Variables|GetLoopTrack) (- (Variables|Variables|GetNumberOfSplinePoints) 1) (- (Variables|Variables|GetNumberOfSplinePoints) 2)))
        (Variables|Variables|SetGlobal_CurrentLoopIndex _index)
        (Variables|Variables|SetDrawLeftGuardRail (.leftguardrail (Utilities|Array|Get(acopy) (Variables|Variables|GetRoadDataArray) (Variables|Variables|GetGlobal_CurrentLoopIndex))))
        (Variables|Variables|SetDrawRightGuardRail (.rightguardrail (Utilities|Array|Get(acopy) (Variables|Variables|GetRoadDataArray) (Variables|Variables|GetGlobal_CurrentLoopIndex))))
        ;[1 1 1] Build Different Road Element based on selected mesh
        (CallFunction|BuildRoadElement (Variables|Variables|GetGlobal_CurrentLoopIndex) (Variables|Mesh|GetRoadMesh))))
    (:then_3
      ;[1 1 1] Draw Current Spline Point Index
      (for _index_2 (range 0 (- (Variables|Variables|GetNumberOfSplinePoints) 1))
        (Variables|Default|SetCurrentIndex _index_2)
        (Utilities|FlowControl|Sequence
          (:then_0
            (if (Variables|Variables|GetShowSplinePointNumbers)
              (Variables|Default|SetCurrentTrackPoint (Utilities|String|ToString(Integer) (Variables|Default|GetCurrentIndex)))
              (bind _returnvalue (AddComponent|AddTextRenderComponent false (Math|Transform|MakeTransform (Math|Vector|MakeVector (.X (Math|Vector|BreakVector (.Location (Spline|GetLocationandTangentatSplinePoint (Variables|Default|GetSpline) (Variables|Default|GetCurrentIndex) "Local")))) (.Y (Math|Vector|BreakVector (.Location (Spline|GetLocationandTangentatSplinePoint (Variables|Default|GetSpline) (Variables|Default|GetCurrentIndex) "Local")))) (+ (.Z (Math|Vector|BreakVector (.Location (Spline|GetLocationandTangentatSplinePoint (Variables|Default|GetSpline) (Variables|Default|GetCurrentIndex) "Local")))) 6e+01)) (Math|Rotator|MakeRotfromX (* (.Tangent (Spline|GetLocationandTangentatSplinePoint (Variables|Default|GetSpline) (Variables|Default|GetCurrentIndex) "Local")) -1)))))
              (Rendering|Components|TextRender|SetText _returnvalue (Utilities|Text|ToText(String) (Variables|Default|GetCurrentTrackPoint)))))
          (:then_1
            ;[1 1 1] Draw Bridge_Support on each point
            (if (Variables|Variables|GetAddSupportOnEachPoint)
              (bind _returnvalue_2 (AddComponent|AddSplineMeshComponent false (Math|Transform|MakeTransform (Math|Vector|MakeVector (+ (.X (Math|Vector|BreakVector (.Location (Spline|GetLocationandTangentatSplinePoint (Variables|Default|GetSpline) (Variables|Default|GetCurrentIndex) "Local")))) _x) (+ (.Y (Math|Vector|BreakVector (.Location (Spline|GetLocationandTangentatSplinePoint (Variables|Default|GetSpline) (Variables|Default|GetCurrentIndex) "Local")))) _y) (+ (.Z (Math|Vector|BreakVector (.Location (Spline|GetLocationandTangentatSplinePoint (Variables|Default|GetSpline) (Variables|Default|GetCurrentIndex) "Local")))) _z)) (Math|Rotator|MakeRotator (+ (.Roll (Math|Rotator|BreakRotator (.bridgesupportrotationoffset (Utilities|Array|Get(acopy) (Variables|Variables|GetRoadDataArray) (Variables|Default|GetCurrentIndex))))) (.Roll (Math|Rotator|BreakRotator (Spline|GetRotationatSplinePoint (Variables|Default|GetSpline) (Variables|Default|GetCurrentIndex) "Local")))) (+ (.Pitch (Math|Rotator|BreakRotator (.bridgesupportrotationoffset (Utilities|Array|Get(acopy) (Variables|Variables|GetRoadDataArray) (Variables|Default|GetCurrentIndex))))) (.Pitch (Math|Rotator|BreakRotator (Spline|GetRotationatSplinePoint (Variables|Default|GetSpline) (Variables|Default|GetCurrentIndex) "Local")))) (+ (.Yaw (Math|Rotator|BreakRotator (.bridgesupportrotationoffset (Utilities|Array|Get(acopy) (Variables|Variables|GetRoadDataArray) (Variables|Default|GetCurrentIndex))))) (.Yaw (Math|Rotator|BreakRotator (Spline|GetRotationatSplinePoint (Variables|Default|GetSpline) (Variables|Default|GetCurrentIndex) "Local"))))) (Variables|Variables|GetBridge_Support_Scale))))
              (bind _output_get_2 (Variables|Default|SetSplineMeshRef _returnvalue_2))
              (Components|StaticMesh|SetStaticMesh _output_get_2 (Variables|Mesh|GetBridge_SupportMesh))
              (SplineMesh|SetStartandEnd (Variables|Default|GetSplineMeshRef) (.bridgesupportoffset (Utilities|Array|Get(acopy) (Variables|Variables|GetRoadDataArray) (Variables|Default|GetCurrentIndex))) (SplineMesh|GetStartTangent (Variables|Default|GetSplineMeshRef)) (SplineMesh|GetEndTangent (Variables|Default|GetSplineMeshRef)) (Math|Vector|MakeVector (+ (.X (Math|Vector|BreakVector (Variables|Variables|GetBridge_Support_Scale))) (.X (Math|Vector|BreakVector (.bridgesupportoffset (Utilities|Array|Get(acopy) (Variables|Variables|GetRoadDataArray) (Variables|Default|GetCurrentIndex)))))) (.Y (Math|Vector|BreakVector (.bridgesupportoffset (Utilities|Array|Get(acopy) (Variables|Variables|GetRoadDataArray) (Variables|Default|GetCurrentIndex))))) (.Z (Math|Vector|BreakVector (.bridgesupportoffset (Utilities|Array|Get(acopy) (Variables|Variables|GetRoadDataArray) (Variables|Default|GetCurrentIndex)))))) true :!class /Script/Engine.SplineMeshComponent)
              (Collision|SetCollisionEnabled (Variables|Default|GetSplineMeshRef) (select (Variables|Variables|GetHaveCollision?) "QueryAndPhysics" "NoCollision")))))))))

(fn BuildRoadElement
  (params (Loop%20Index :type Integer) (RoadElementMesh :type Static%20Mesh%20Object%20Reference))
  ;[1 1 1] Store Next Index
  (LocalVariables|SetCurrentLoopIndex Loop%20Index)
  (LocalVariables|SetNextLoopIndex (Math|Integer|%(Integer) (+ Loop%20Index 1) (Variables|Variables|GetNumberOfSplinePoints)))
  (LocalVariables|SetLocal_RoadElementMesh RoadElementMesh)
  (Utilities|FlowControl|Sequence
    (:then_0
      ;[1 1 1] Store Spline informations
      (LocalVariables|SetStartLocation (.Location (Spline|GetLocationandTangentatSplinePoint (Variables|Default|GetSpline) (LocalVariables|GetCurrentLoopIndex) (select (Variables|Variables|GetUseWorldSpaceCoordinate) "World" "Local"))))
      (LocalVariables|SetTangentStartLocation (.Tangent (Spline|GetLocationandTangentatSplinePoint (Variables|Default|GetSpline) (LocalVariables|GetCurrentLoopIndex) (select (Variables|Variables|GetUseWorldSpaceCoordinate) "World" "Local"))))
      (LocalVariables|SetEndLocation (.Location (Spline|GetLocationandTangentatSplinePoint (Variables|Default|GetSpline) (LocalVariables|GetNextLoopIndex) (select (Variables|Variables|GetUseWorldSpaceCoordinate) "World" "Local"))))
      (LocalVariables|SetTangentEndLocation (.Tangent (Spline|GetLocationandTangentatSplinePoint (Variables|Default|GetSpline) (LocalVariables|GetNextLoopIndex) (select (Variables|Variables|GetUseWorldSpaceCoordinate) "World" "Local"))))
      (LocalVariables|SetStartRoll (.trackbank (Utilities|Array|Get(acopy) (Variables|Variables|GetRoadDataArray) (LocalVariables|GetCurrentLoopIndex))))
      (LocalVariables|SetRoadStartScale (Math|Vector2D|MakeVector2D (.trackwidth (Utilities|Array|Get(acopy) (Variables|Variables|GetRoadDataArray) (LocalVariables|GetCurrentLoopIndex))) (.trackthickness (Utilities|Array|Get(acopy) (Variables|Variables|GetRoadDataArray) (LocalVariables|GetCurrentLoopIndex)))))
      (LocalVariables|SetEndRoll (.trackbank (Utilities|Array|Get(acopy) (Variables|Variables|GetRoadDataArray) (LocalVariables|GetNextLoopIndex))))
      (LocalVariables|SetRoadEndScale (Math|Vector2D|MakeVector2D (.trackwidth (Utilities|Array|Get(acopy) (Variables|Variables|GetRoadDataArray) (LocalVariables|GetNextLoopIndex))) (.trackthickness (Utilities|Array|Get(acopy) (Variables|Variables|GetRoadDataArray) (LocalVariables|GetNextLoopIndex))))))
    (:then_1
      ;[1 1 1] Build Static Mesh based on Spline datas
      (bind _returnvalue (AddComponent|AddSplineMeshComponent false))
      (bind _output_get (LocalVariables|SetCurentSplineMesh _returnvalue))
      (Components|StaticMesh|SetStaticMesh _output_get (LocalVariables|GetLocal_RoadElementMesh))
      (SplineMesh|SetStartandEnd (LocalVariables|GetCurentSplineMesh) (LocalVariables|GetStartLocation) (LocalVariables|GetTangentStartLocation) (LocalVariables|GetEndLocation) (LocalVariables|GetTangentEndLocation) true :!class /Script/Engine.SplineMeshComponent)
      (Class|SplineMeshComponent|SetStartRoll (LocalVariables|GetCurentSplineMesh) (LocalVariables|GetStartRoll) true)
      (Class|SplineMeshComponent|SetEndRoll (LocalVariables|GetCurentSplineMesh) (LocalVariables|GetEndRoll) true)
      (SplineMesh|SetStartScale (LocalVariables|GetCurentSplineMesh) (LocalVariables|GetRoadStartScale) true :!class /Script/Engine.SplineMeshComponent)
      (SplineMesh|SetEndScale (LocalVariables|GetCurentSplineMesh) (LocalVariables|GetRoadEndScale) true :!class /Script/Engine.SplineMeshComponent)
      (Collision|SetCollisionEnabled (LocalVariables|GetCurentSplineMesh) (select (Variables|Variables|GetHaveCollision?) "QueryAndPhysics" "NoCollision")))))